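; BP_EnemyChaserSpawner is a spawner actor that repeatedly spawns waves of a configurable enemy class at its own transform.
; On BeginPlay it calls SpawnEnemy, which spawns NumberOfEnemies actors at once at the same transform.
; After SpawnDelay, the event calls itself with the spawner's current transform, forming an endless timed loop with no stop condition.
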(event `self.ReceiveBeginPlay`
  (`self.Spawn Enemy` (`self.Enemy`) (`self.GetTransform`) (`self.Number Of Enemies`)))

(event `Spawn Enemy`
  (params (Enemy :type "Actor Class Reference") (`Spawn Transform` :type "Transform Structure") (`Number of enemies` :type Integer))
  (for _ (range `Number of enemies`)
    (`|SpawnActorFromClass` Enemy `Spawn Transform` "Undefined" "OverrideRootScale" null null))
  (`KismetSystemLibrary.Delay` (`self.Spawn Delay`))
  (`self.Spawn Enemy` (`self.Enemy`) (`self.GetTransform`) (`self.Number Of Enemies`)))

(fn `UserConstructionScript`)