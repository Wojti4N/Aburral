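; BP_BulletEnemy is an enemy projectile that damages the player on contact.
; Its Box overlap ignores the instigator and reacts only to actors tagged Player, subtracting DMG directly from the HP of BP_ThirdPersonCharacter.
; The bullet destroys itself after any such tagged overlap, even if the character cast fails.
; A disconnected, disabled game-over widget and pause sequence remains in the graph.
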(event `self.Box.OnComponentBeginOverlap`
  (params (OverlappedComponent :type "PrimitiveComponent Object Reference") (OtherActor :type "Actor Object Reference") (OtherComp :type "PrimitiveComponent Object Reference") (OtherBodyIndex :type Integer) (bFromSweep :type Boolean) (SweepResult :type "HitResult Structure (by ref)"))
  ;[1 1 1] Bullet damage
  (if (!= OtherActor (`self.GetInstigator`))
    (if (`self.ActorHasTag` OtherActor "Player")
      (bind _asbp_third_person_character (cast `/Game/ThirdPerson/Blueprints/BP_ThirdPersonCharacter` OtherActor)
        (:`then`
          (set `/Game/ThirdPerson/Blueprints/BP_ThirdPersonCharacter.HP` (- (`/Game/ThirdPerson/Blueprints/BP_ThirdPersonCharacter.HP` _asbp_third_person_character) (`self.DMG`)) _asbp_third_person_character)
          (`self.K2_DestroyActor`))
        (:`CastFailed`
          (`self.K2_DestroyActor`))))))

(fn `UserConstructionScript`)